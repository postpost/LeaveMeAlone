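; Player controller for LeaveMeAlone that opens the pause menu when the Pause input action is pressed.
; If not already paused, it sets the OnPause flag, pauses the game, and creates and displays a WBP_Pause widget.
; It then switches to UI-only input focused on that widget and shows the mouse cursor.
; This graph contains no unpause logic.
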(event `InputAction|Pause`
  (params (Key :type "Key Structure"))
  (:`Pressed`
    (if (not (`self.OnPause`))
      (bind _output_get (set `self.OnPause` true))
      (`GameplayStatics.SetGamePaused` _output_get)
      (bind _returnvalue (`|CreateWidget` "/Game/LeaveMeAlone/Widgets/UI/WBP_Pause.WBP_Pause_C"))
      (bind _output_get_2 (set `self.PauseWidget` _returnvalue))
      (`UserWidget.AddToViewport` _output_get_2 0)
      (`WidgetBlueprintLibrary.SetInputMode_UIOnlyEx` self (`self.PauseWidget`))
      (set `self.bShowMouseCursor` true))))

(fn `UserConstructionScript`)