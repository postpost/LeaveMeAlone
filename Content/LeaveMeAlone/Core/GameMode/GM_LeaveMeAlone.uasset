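; GM_LeaveMeAlone is a game mode that runs the match countdown and ends play on timeout.
; BeginPlay starts a looping one-second timer that calls DecreaseTime to decrement GameTime.
; When GameTime reaches zero, it clears the timer and opens TimeoutLevel.
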(event `self.ReceiveBeginPlay`
  (bind _returnvalue (`KismetSystemLibrary.K2_SetTimerDelegate` (delegate `DecreaseTime`) 1.0 true))
  (set `self.GameTimerHandle` _returnvalue))

(event `DecreaseTime`
  (bind _output_get (set `self.GameTime` (- (`self.GameTime`) 1)))
  (if (== _output_get 0)
    (`KismetSystemLibrary.K2_ClearAndInvalidateTimerHandle` (`self.GameTimerHandle`))
    (`GameplayStatics.OpenLevelBySoftObjectPtr` "/Game/LeaveMeAlone/Levels/TimeoutLevel.TimeoutLevel")))

(fn `UserConstructionScript`)